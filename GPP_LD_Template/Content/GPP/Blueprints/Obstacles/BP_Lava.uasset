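; BP_Lava is an obstacle that kills the player on contact unless it is frozen.
; On BeginPlay it creates a dynamic material instance for its mesh and hands it to BPFreezableComponent, then initialises the freeze status.
; When the mesh is hit by a BP_PlayerCharacter, it queries the component's frozen state and calls KillPlayer if not frozen.
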(event OnComponentHit(Mesh)
  (params (HitComponent :type Primitive%20Component%20Object%20Reference) (OtherActor :type Actor%20Object%20Reference) (OtherComp :type Primitive%20Component%20Object%20Reference) (NormalImpulse :type Vector :default "0, 0, 0") (Hit :type Hit%20Result%20Structure%20%28by%20ref%29))
  ;[0.4491 0.8591 1] Check if player collides and then kill the player
  (bind _asbp_player_character (Utilities|Casting|CastToBP_PlayerCharacter OtherActor))
  (if (CallFunction|IsNotFrozen)
    (Default|KillPlayer _asbp_player_character)
    (Development|PrintString "Killing Player")))

(event EventBeginPlay
  (bind _mesh (Variables|Default|GetMesh))
  (bind _bp_freezablecomponent (Variables|Default|GetBP_FreezableComponent))
  ;[0.4491 0.8591 1] Initialise freeze component
  (bind _returnvalue (Rendering|Material|CreateDynamicMaterialInstance (Rendering|Material|GetMaterial _mesh 0) "None" "None" :!class /Script/Engine.KismetMaterialLibrary))
  (Rendering|Material|SetMaterial _mesh 0 _returnvalue)
  (Default|InitMaterial _bp_freezablecomponent (Utilities|Array|MakeArray _returnvalue))
  (Default|InitFreezeStatus _bp_freezablecomponent))

(fn ConstructionScript)

(fn IsNotFrozen
  (return (not (Default|GetIsFrozen (Variables|Default|GetBP_FreezableComponent)))))